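; BP_MagicPlayerController is the player controller that handles team selection and spawn requests for the Magic game mode.
; On BeginPlay the server possesses the first BP_MagicEmptyPawn found in the level, while the local controller shows the WBP_TeamSelect widget.
; The TeamSelected event forwards the chosen team and the controller to BP_MagicGameMode's RequestSpawn.
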(event `self.ReceiveBeginPlay`
  (`|ExecutionSequence`
    (:`then_0`
      (`/Engine/EditorBlueprintResources/ActorMacros.Switch Has Authority`
        (:`Authority`
          (bind _outactors (`GameplayStatics.GetAllActorsOfClass` "/Game/Game/BP_MagicEmptyPawn.BP_MagicEmptyPawn_C"))
          (`self.Possess` (`|GetArrayItem` _outactors)))))
    (:`then_1`
      (if (`self.IsLocalController`)
        (bind _returnvalue (`|CreateWidget` "/Game/UI/WBP_TeamSelect.WBP_TeamSelect_C"))
        (`UserWidget.AddToViewport` _returnvalue 0)))))

(event `TeamSelected`
  (params (Team :type "ETeams Enum" :default "None"))
  (`/Game/Game/BP_MagicGameMode.RequestSpawn` (cast `/Game/Game/BP_MagicGameMode` (`GameplayStatics.GetGameMode`) :!pure true) Team self))

(fn `UserConstructionScript`)